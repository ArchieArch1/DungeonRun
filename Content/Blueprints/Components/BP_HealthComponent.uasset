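; Health component that tracks damage on its owning actor and handles player death and scoring.
; On BeginPlay it caches game and player references and binds to the owner's any-damage event.
; Hits instigated by a player controller reduce and print Health.
; At zero, a player owner is unpossessed and destroyed, and the game mode increments the score with victim and instigator controllers; Defeat is an empty stub.
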(event `self.ReceiveBeginPlay`
  (bind _returnvalue (`self.GetOwner`))
  (bind _asbp_game_mode_base (cast `/Game/Blueprints/BP_GameModeBase` (`GameplayStatics.GetGameMode`)))
  (set `self.GameModeRef` _asbp_game_mode_base)
  (bind _asdr_game_state_base (cast `DR_GameStateBase` (`GameplayStatics.GetGameState`)))
  (set `self.GameStateRef` _asdr_game_state_base)
  (add `Actor.OnTakeAnyDamage` _returnvalue (delegate `OnTakeAnyDamage_Event_0`))
  (bind _asbp_player (cast `/Game/Blueprints/Player/BP_Player` _returnvalue))
  (set `self.PlayerRef` _asbp_player)
  (bind _asbp_player_controller (cast `/Game/Blueprints/Player/BP_PlayerController` (`Pawn.GetController` (`self.PlayerRef`))))
  (set `self.PlayerControllerRef` _asbp_player_controller))

(event `OnTakeAnyDamage_Event_0`
  (params (DamagedActor :type "Actor Object Reference") (Damage :type "Float (double-precision)") (DamageType :type "DamageType Object Reference") (InstigatedBy :type "Controller Object Reference") (DamageCauser :type "Actor Object Reference"))
  (bind _asbp_player_controller (cast `/Game/Blueprints/Player/BP_PlayerController` InstigatedBy))
  (set `self.InstigatorControllerRef` _asbp_player_controller)
  ;[0 0 0] Damage interface is probably better
  (bind _asbp_player (cast `/Game/Blueprints/Player/BP_Player` (`self.GetOwner`))
    (:`then`
      (set `self.DamagedCharacter` _asbp_player)
      (set `self.bIsCharacter` true))
    (:`CastFailed`
      (set `self.bIsCharacter` false)))
  (`self.TakeDamage` Damage))

(fn `Defeat`
  (params (InstigatedControllerRef :type "DR_PlayerController Object Reference")))

(fn `TakeDamage`
  (params (DamageAmount :type "Float (double-precision)") (Instigator :type "/Game/Blueprints/Player/BP_PlayerController Object Reference"))
  (bind _playercontrollerref (`self.PlayerControllerRef`))
  (bind _output_get (set `self.Health` (- (`self.Health`) DamageAmount)))
  (`KismetSystemLibrary.PrintString` (`KismetStringLibrary.Conv_DoubleToString` _output_get))
  (if (and (`self.bIsCharacter`) (<= (`self.Health`) 0.0))
    (`Controller.UnPossess` _playercontrollerref)
    (`Actor.K2_DestroyActor` (`self.PlayerRef`))
    (`/Game/Blueprints/BP_GameModeBase.ServerIncrementScore` (`self.GameModeRef`) _playercontrollerref (`self.InstigatorControllerRef`))))
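; Player controller that creates the HUD for the local player and routes respawn and score requests to the game mode.
; On BeginPlay, where the game mode is valid, it caches game mode and game state and binds countdown and round timer updates to the HUD.
; The Respawn input works only without a possessed pawn and calls the game mode on authority.
; IncrementScore forwards both controllers to the game mode.
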(event `self.ReceiveBeginPlay`
  (bind _returnvalue (`GameplayStatics.GetGameMode`))
  (if (`self.IsLocalController`)
    (bind _returnvalue_2 (`|CreateWidget` "/Game/Blueprints/UI/WBP_HUD.WBP_HUD_C" self))
    (bind _output_get (set `self.HUD` _returnvalue_2))
    (`UserWidget.AddToViewport` _output_get 0)
    (`/Engine/EditorBlueprintResources/StandardMacros.IsValid` _returnvalue
      (:`Is Valid`
        (bind _asbp_game_mode_base (cast `/Game/Blueprints/BP_GameModeBase` _returnvalue))
        (set `self.BPGameModeRef` _asbp_game_mode_base)
        (bind _asdr_game_state_base (cast `DR_GameStateBase` (`GameplayStatics.GetGameState`)))
        (set `self.BPGameStateRef` _asdr_game_state_base)
        (add `DR_GameStateBase.FOnUpdateStartTimerWidget` (`self.BPGameStateRef`) (delegate `StartCountdown`))
        (add `DR_GameStateBase.FOnUpdateRoundTimerWidget` (`self.BPGameStateRef`) (delegate `FOnUpdateRoundTimerWidget_Event_0`))))))

(event `StartCountdown`
  (`/Game/Blueprints/UI/WBP_HUD.UpdateCountdownTimer` (`self.HUD`) (`DR_GameStateBase.StartCountdownDuration` (`self.BPGameStateRef`))))

(event `FOnUpdateRoundTimerWidget_Event_0`
  (`/Game/Blueprints/UI/WBP_HUD.UpdateGameTimer` (`self.HUD`) (`DR_GameStateBase.RemainingRoundTime` (`self.BPGameStateRef`))))

(event `InputAction|Respawn`
  (params (Key :type "Key Structure"))
  (:`Pressed`
    (`/Engine/EditorBlueprintResources/StandardMacros.IsValid` (`self.K2_GetPawn` self)
      (:`Is Valid`
        (`KismetSystemLibrary.PrintString` "Controller is still possessing a pawn"))
      (:`Is Not Valid`
        (`self.RequestGameModeRespawn`)))))

(event `RequestGameModeRespawn`
  (bind _bpgamemoderef (`self.BPGameModeRef`))
  (`/Engine/EditorBlueprintResources/ActorMacros.Switch Has Authority`
    (:`Authority`
      (`/Engine/EditorBlueprintResources/StandardMacros.IsValid` _bpgamemoderef
        (:`Is Valid`
          (`/Game/Blueprints/BP_GameModeBase.Respawn` _bpgamemoderef self))))))

(event `IncrementScore`
  (params (OpponentController :type "/Game/Blueprints/Player/BP_PlayerController Object Reference"))
  (`/Game/Blueprints/BP_GameModeBase.ServerIncrementScore` (`self.BPGameModeRef`) self OpponentController))

(fn `Countdown`)

(fn `UserConstructionScript`)